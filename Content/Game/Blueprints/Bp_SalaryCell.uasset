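; Salary cell Blueprint that pays the player money when activated.
; On BeginPlay it caches the Bp_LoopGameInstance.
; Its Activate event adds SalaryValue to the instance's Money, then calls TestEnd on that instance.
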(event `self.ReceiveBeginPlay`
  (`parent.ReceiveBeginPlay`)
  (bind _asbp_loop_game_instance (cast `/Game/Game/GameInstance/Bp_LoopGameInstance` (`GameplayStatics.GetGameInstance`)))
  (set `self.As Bp Loop Game Instance_0` _asbp_loop_game_instance))

(event `/Game/Game/Blueprints/BPI_Activable.Activate`
  (params (Pawn :type "/Game/Game/Blueprints/BP_Pawn Object Reference"))
  (bind _as_bp_loop_game_instance_0 (`self.As Bp Loop Game Instance_0`))
  (set `/Game/Game/GameInstance/Bp_LoopGameInstance.Money` (+ (`self.SalaryValue`) (`/Game/Game/GameInstance/Bp_LoopGameInstance.Money` _as_bp_loop_game_instance_0)) _as_bp_loop_game_instance_0)
  (`/Game/Game/GameInstance/Bp_LoopGameInstance.TestEnd` _as_bp_loop_game_instance_0))

(fn `UserConstructionScript`
  (`parent.UserConstructionScript`))