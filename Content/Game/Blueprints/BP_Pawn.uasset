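; BP_Pawn is the player's board-game piece, which moves between numbered cells on a Board.
; On BeginPlay it snaps to the cell number stored in Bp_LoopGameInstance and creates the dialogue and dice-button widgets.
; TryMoving adds a value to that number, lets the Board resolve the destination, stores it, then teleports and activates the cell.
; UpdateCell asks the current cell to update its message.
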(event `self.ReceiveBeginPlay`
  (bind _asbp_loop_game_instance (cast `/Game/Game/GameInstance/Bp_LoopGameInstance` (`GameplayStatics.GetGameInstance`)))
  (set `self.As Bp Loop Game Instance` _asbp_loop_game_instance)
  (`self.MoveToCell`)
  (bind _returnvalue (`|CreateWidget` "/Game/Game/Widget/WBP_DialogueUi.WBP_DialogueUi_C"))
  (bind _output_get (set `self.Wbp_Dialogue` _returnvalue))
  (set `/Game/Game/Widget/WBP_DialogueUi.Pawn` self _output_get)
  (`UserWidget.AddToViewport` _output_get 0)
  (bind _returnvalue_2 (`|CreateWidget` "/Game/Game/Widget/WBP_DiceButton.WBP_DiceButton_C"))
  (bind _output_get_2 (set `self.WBP_DiceButton` _returnvalue_2))
  (set `/Game/Game/Widget/WBP_DiceButton.Dice` (`self.Bp_Dice`) _output_get_2)
  (`UserWidget.AddToViewport` _output_get_2 0))

(fn `ActivateCell`
  (bind _cell (`/Game/Game/Blueprints/BP_Board.GetCellByNumber` (`self.Board`) (`/Game/Game/GameInstance/Bp_LoopGameInstance.CellNumber` (`self.As Bp Loop Game Instance`))))
  (`/Game/Game/Blueprints/BP_Cell.Activate` _cell self))

(fn `MoveToCell`
  (bind _cell (`/Game/Game/Blueprints/BP_Board.GetCellByNumber` (`self.Board`) (`/Game/Game/GameInstance/Bp_LoopGameInstance.CellNumber` (`self.As Bp Loop Game Instance`))))
  (bind (_returnvalue_location _returnvalue_rotation) (`KismetMathLibrary.BreakTransform` (`self.GetTransform` _cell)))
  (`self.K2_SetActorLocation` _returnvalue_location)
  (`self.K2_SetActorRotation` _returnvalue_rotation))

(fn `TryMoving`
  (params (value :type Integer))
  (bind _as_bp_loop_game_instance (`self.As Bp Loop Game Instance`))
  (bind _cell_ (`/Game/Game/Blueprints/BP_Board.GetNextCellToMove` (`self.Board`) (+ value (`/Game/Game/GameInstance/Bp_LoopGameInstance.CellNumber` _as_bp_loop_game_instance))))
  (set `/Game/Game/GameInstance/Bp_LoopGameInstance.CellNumber` _cell_ _as_bp_loop_game_instance)
  (`self.MoveToCell`)
  (`self.ActivateCell`))

(fn `UpdateCell`
  (bind _cell (`/Game/Game/Blueprints/BP_Board.GetCellByNumber` (`self.Board`) (`/Game/Game/GameInstance/Bp_LoopGameInstance.CellNumber` (`self.As Bp Loop Game Instance`))))
  (message `/Game/Game/Blueprints/BPI_Activable.Update` _cell self))

(fn `UserConstructionScript`)