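; BP_DialogueCell is an actor that runs a dialogue sequence on the given pawn's dialogue widget.
; Activate loads the current row from its dialogue component, pushes the character and long text to the pawn's WbpDialogue, then starts it.
; Each Update call either ends the dialogue when the component reports it finished, or advances to the next row and refreshes the widget.
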(event `/Game/Game/Blueprints/BPI_Activable.Activate`
  (params (Pawn :type "/Game/Game/Blueprints/BP_Pawn Object Reference"))
  (bind _wbp_dialogue (`/Game/Game/Blueprints/BP_Pawn.Wbp_Dialogue` Pawn))
  (bind _bpc_dialoguecomponent (`self.BPC_DialogueComponent`))
  (`/Game/Game/DataTable/BPC_DialogueComponent.GetCurrentDialogueRowData` _bpc_dialoguecomponent)
  (bind _character (`/Game/Game/DataTable/BPC_DialogueComponent.GetCharacterFromRow` _bpc_dialoguecomponent))
  (bind _dialoguelong (`/Game/Game/DataTable/BPC_DialogueComponent.GetDialogueLongFromCurrentRow` _bpc_dialoguecomponent))
  (`/Game/Game/Widget/WBP_DialogueUi.UpdateDialogue` _wbp_dialogue _character _dialoguelong "")
  (`/Game/Game/Widget/WBP_DialogueUi.StartDialogue` _wbp_dialogue))

(event `/Game/Game/Blueprints/BPI_Activable.Update`
  (params (Pawn :type "/Game/Game/Blueprints/BP_Pawn Object Reference"))
  (bind _bpc_dialoguecomponent (`self.BPC_DialogueComponent`))
  (bind _wbp_dialogue (`/Game/Game/Blueprints/BP_Pawn.Wbp_Dialogue` Pawn))
  (bind _isfinished (`/Game/Game/DataTable/BPC_DialogueComponent.IsDialogueFinished` _bpc_dialoguecomponent))
  (if _isfinished
    (`/Game/Game/Widget/WBP_DialogueUi.EndDialogue` _wbp_dialogue)
    (else
      (`/Game/Game/DataTable/BPC_DialogueComponent.ReadNextRow` _bpc_dialoguecomponent)
      (bind _character (`/Game/Game/DataTable/BPC_DialogueComponent.GetCharacterFromRow` _bpc_dialoguecomponent))
      (bind _dialoguelong (`/Game/Game/DataTable/BPC_DialogueComponent.GetDialogueLongFromCurrentRow` _bpc_dialoguecomponent))
      (`/Game/Game/Widget/WBP_DialogueUi.UpdateDialogue` _wbp_dialogue _character _dialoguelong ""))))

(fn `UserConstructionScript`
  (`parent.UserConstructionScript`))