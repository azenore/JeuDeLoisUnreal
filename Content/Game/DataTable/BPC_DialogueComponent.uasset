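; Dialogue component that steps through conversation rows stored in a data table.
; It looks up rows by the current row number converted to a name and caches the result for the text, character and end-of-dialogue getters.
; Each row links to the next, with a negative next index marking the end.
; An optional alternative row allows branching, falling back to the next row when set to zero.
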(fn `GetCharacterFromRow`
  (returns (Character :type String))
  (return (`.Character_5_6739AB1E427D194D66C29BA8F5AEEEE6` (break `/Game/Game/DataTable/ST_DialogueRowDatas` (`self.CurrentDialgueRow`)))))

(fn `GetCurrentDialogueRowData`
  (returns (RowData :type "/Game/Game/DataTable/ST_DialogueRowDatas Structure"))
  (bind _returnvalue (`|GetDataTableRow` (`self.DialogueDataTable`) (`KismetStringLibrary.Conv_StringToName` (`KismetStringLibrary.Conv_IntToString` (`self.CurrentRowNumber`))))
    (:`then`
      (bind _output_get (set `self.CurrentDialgueRow` _returnvalue))
      (return _output_get))))

(fn `GetDialogueLongFromCurrentRow`
  (returns (DialogueLong :type String))
  (return (`.DialogueLong_11_0509333A43ABC1DF2FD9DBA9F72D30CD` (break `/Game/Game/DataTable/ST_DialogueRowDatas` (`self.CurrentDialgueRow`)))))

(fn `IsDialogueFinished`
  (returns (IsFinished :type Boolean))
  (return (<= (`.NextRow_10_BBE19779419715D59035A1840551724F` (break `/Game/Game/DataTable/ST_DialogueRowDatas` (`self.CurrentDialgueRow`))) -1)))

(fn `ReadAlternativeRow`
  (bind (_rownumber _character _dialoguelong _nextrow _alternativerow) (break `/Game/Game/DataTable/ST_DialogueRowDatas` (`self.CurrentDialgueRow`)))
  (if (!= _alternativerow 0)
    (set `self.CurrentRowNumber` _alternativerow)
    (`self.GetCurrentDialogueRowData`)
    (else
      (`self.ReadNextRow`))))

(fn `ReadNextRow`
  (set `self.CurrentRowNumber` (`.NextRow_10_BBE19779419715D59035A1840551724F` (break `/Game/Game/DataTable/ST_DialogueRowDatas` (`self.CurrentDialgueRow`))))
  (`self.GetCurrentDialogueRowData`))